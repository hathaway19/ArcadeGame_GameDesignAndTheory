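; Teleporter powerup that sends any actor overlapping its capsule to the currently stored destination.
; Player1Bullets pass through to that destination without changing it, while any other actor also triggers a random pick from four TeleportLocations entries.
; A particle emitter marks each newly picked destination, with FirstTime and CountTele selecting which stored emitter to destroy before spawning the next.
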(event OnComponentBeginOverlap(Capsule)
  (params (OverlappedComponent :type Primitive%20Component%20Object%20Reference) (OtherActor :type Actor%20Object%20Reference) (OtherComp :type Primitive%20Component%20Object%20Reference) (OtherBodyIndex :type Integer) (bFromSweep :type Boolean) (SweepResult :type Hit%20Result%20Structure%20%28by%20ref%29))
  (if (Variables|Default|GetFirstTime)
    (bind _asplayer_1bullets (Utilities|Casting|CastToPlayer1Bullets OtherActor)
      (:then
        (Transformation|Teleport _asplayer_1bullets (Variables|Default|GetToTeleport) "0, 0, 0"))
      (:CastFailed
        (Transformation|Teleport OtherActor (Variables|Default|GetToTeleport) "0, 0, 0")
        (Variables|Default|SetFirstTime false)
        (bind _output_get (Variables|Default|SetToTeleport (Utilities|Array|Get(acopy) (Variables|Default|GetTeleportLocations) (Math|Random|RandomInteger 4))))
        (Variables|Default|SetCountTele 1)
        (bind _returnvalue (Effects|SpawnEmitteratLocation "/Game/StarterContent/Particles/TeleportLocation.TeleportLocation" _output_get))
        (Variables|Default|SetNewVar_1 _returnvalue)))
    (else
      (bind _asplayer_1bullets_2 (Utilities|Casting|CastToPlayer1Bullets OtherActor)
        (:then
          (Transformation|Teleport _asplayer_1bullets_2 (Variables|Default|GetToTeleport) "0, 0, 0"))
        (:CastFailed
          (Transformation|Teleport OtherActor (Variables|Default|GetToTeleport) "0, 0, 0")
          (bind _output_get_2 (Variables|Default|SetToTeleport (Utilities|Array|Get(acopy) (Variables|Default|GetTeleportLocations) (Math|Random|RandomInteger 4))))
          (if (== (Variables|Default|GetCountTele) 2)
            (Components|DestroyComponent (Variables|Default|GetNewVar_0))
            (else
              (Components|DestroyComponent (Variables|Default|GetNewVar_1))))
          (bind _returnvalue_2 (Effects|SpawnEmitteratLocation "/Game/StarterContent/Particles/TeleportLocation.TeleportLocation" _output_get_2))
          (Variables|Default|SetNewVar_0 _returnvalue_2)
          (Variables|Default|SetCountTele 2))))))

(event EventTick
  (params (DeltaSeconds :type Float%20%28single-precision%29)))

(event EventBeginPlay)

(fn ConstructionScript)