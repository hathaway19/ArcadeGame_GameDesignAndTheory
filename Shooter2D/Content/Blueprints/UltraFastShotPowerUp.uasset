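; UltraFastShotPowerUp is a pickup that sets the BulletsLeft count on the RedAlien or BlueAlien that touches it.
; A capsule overlap identifies the alien by cast, then destroys the capsule and Paper2D sprite components while leaving the actor alive.
; The surviving actor waits through a delay, then calls FastBullet on the mainGameMode.
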(event OnComponentBeginOverlap(Capsule)
  (params (OverlappedComponent :type Primitive%20Component%20Object%20Reference) (OtherActor :type Actor%20Object%20Reference) (OtherComp :type Primitive%20Component%20Object%20Reference) (OtherBodyIndex :type Integer) (bFromSweep :type Boolean) (SweepResult :type Hit%20Result%20Structure%20%28by%20ref%29))
  (bind _capsule (Variables|Default|GetCapsule))
  (bind _asred_alien (Utilities|Casting|CastToRedAlien OtherActor)
    (:then
      (Variables|/Game/Blueprints/RedAlien.RedAlien_C|SetbulletsLeft _asred_alien 5.0)
      (Components|DestroyComponent _capsule))
    (:CastFailed
      (bind _asblue_alien (Utilities|Casting|CastToBlueAlien OtherActor))
      (Variables|/Game/Blueprints/BlueAlien.BlueAlien_C|SetbulletsLeft _asblue_alien 5.0)
      (Components|DestroyComponent _capsule)))
  (bind _asmain_game_mode (Utilities|Casting|CastTomainGameMode (Game|GetGameMode)))
  (Utilities|FlowControl|Delay 2e+01)
  (Default|FastBullet _asmain_game_mode))

(event EventBeginPlay)

(event EventTick
  (params (DeltaSeconds :type Float%20%28single-precision%29)))

(fn ConstructionScript)