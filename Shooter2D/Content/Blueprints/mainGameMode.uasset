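; Game mode for a two-player local match that sets up the HUD, a start countdown and powerup spawns.
; On BeginPlay it creates the second player, disables both players' input and loops a one-second delay until the countdown ends.
; It then restores input, spawns a teleport powerup with a random destination and, after a random delay, a fast-shot powerup.
; Tick converts the countdown to text for the HUD.
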(event EventBeginPlay
  (bind _returnvalue (Game|GetPlayerCharacter 1))
  (bind _returnvalue_2 (Game|GetPlayerCharacter 0))
  ;[1 1 1] Display HUD
  (Class|GameplayStatics|CreatePlayer 1)
  (bind _returnvalue_3 (UserInterface|CreateWidget "/Game/Blueprints/UI/dontDelete/myHUD.myHUD_C"))
  (Variables|Default|SetHUDReference _returnvalue_3)
  (UserInterface|Viewport|AddtoViewport _returnvalue_3 0)
  ;[1 1 1] Disables player controls untill countdown is completed
  (Input|DisableInput _returnvalue_2 (Game|GetPlayerController 0))
  (Input|DisableInput _returnvalue (Game|GetPlayerController 1))
  (Variables|Default|SetsetCountDownVisible "Visible")
  (Utilities|FlowControl|Delay 1.0 :!label _label)
  (if (== (Variables|Default|GetintCountDown) 0)
    (Input|EnableInput _returnvalue_2 (Game|GetPlayerController 0))
    (Input|EnableInput _returnvalue (Game|GetPlayerController 1))
    (Variables|Default|SetsetCountDownVisible "Hidden")
    (CallFunction|Spawnteleport)
    (Utilities|FlowControl|Delay (Math|Conversions|ToFloat(Integer) (Math|Random|RandomInteger 30)))
    (CallFunction|FastBullet)
    (else
      (Variables|Default|SetintCountDown (- (Variables|Default|GetintCountDown) 1))
      (goto _label))))

(event EventTick
  (params (DeltaSeconds :type Float%20%28single-precision%29))
  ;[1 1 1] Updates text for UI
  (CallFunction|InitText))

(fn ConstructionScript)

(fn InitText
  ;[1 1 1] Converts Variables to Text for HUD
  (Variables|Default|SetCountDownText (Utilities|Text|ToText(Integer) (Variables|Default|GetintCountDown))))

(fn Spawnteleport
  (bind _returnvalue (Game|SpawnActorfromClass "/Game/Blueprints/TeleportPowerup.TeleportPowerup_C" (Math|Transform|MakeTransform (Math|Vector|MakeVector 9.5e+02 0.0 1.38e+03)) "AdjustIfPossibleButAlwaysSpawn" 0 0))
  (Variables|/Game/Blueprints/TeleportPowerup.TeleportPowerup_C|SetToTeleport _returnvalue (Utilities|Array|Get(acopy) (Variables|/Game/Blueprints/TeleportPowerup.TeleportPowerup_C|GetTeleportLocations _returnvalue) (Math|Random|RandomInteger 4))))

(fn FastBullet
  (Game|SpawnActorfromClass "/Game/Blueprints/UltraFastShotPowerUp.UltraFastShotPowerUp_C" (Math|Transform|MakeTransform (Math|Vector|MakeVector 9.6e+02 0.0 9.5e+02)) "AdjustIfPossibleButAlwaysSpawn" 0 0))