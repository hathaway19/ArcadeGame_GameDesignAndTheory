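; RedAlien is a side-view flipbook player character for a two-player shooter, despite using BlueAlien flipbooks.
; It fires forward or up via PointUp input, with bullets inheriting some character velocity and a timeline refilling ammo.
; Tick feeds movement and shooting state to AnimationPicker, while a CanJumpInternal override enables multi-jumping.
; Player1Bullets hits drain health; at zero it increments BlueWins, shows P1win, disables input and opens NewLevel.
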(event OnComponentHit(CapsuleComponent)
  (params (HitComponent :type Primitive%20Component%20Object%20Reference) (OtherActor :type Actor%20Object%20Reference) (OtherComp :type Primitive%20Component%20Object%20Reference) (NormalImpulse :type Vector :default "0, 0, 0") (Hit :type Hit%20Result%20Structure%20%28by%20ref%29))
  (bind _returnvalue (Transformation|GetActorLocation))
  ;[1 1 1] When a bullet hits alien, QUITS GAME AFTER BEING HIT 4 TIMES
  (bind _asplayer_1bullets (Utilities|Casting|CastToPlayer1Bullets OtherActor))
  (Effects|SpawnEmitteratLocation "/Game/StarterContent/Particles/PlayerHit.PlayerHit" _returnvalue)
  (Actor|DestroyActor _asplayer_1bullets)
  (Audio|SpawnSoundatLocation "/Game/SoundAssets/Impact.Impact" _returnvalue)
  (bind _output_get (Variables|Default|SethealthLeft (- (Variables|Default|GethealthLeft) 25.0)))
  (if (== _output_get 0.0)
    (Utilities|FlowControl|Sequence
      (:then_0
        (bind _asmy_game_instance (Utilities|Casting|CastTomyGameInstance (Game|GetGameInstance)))
        (Variables|/Game/Blueprints/myGameInstance.myGameInstance_C|SetBlueWins _asmy_game_instance (+ (Variables|/Game/Blueprints/myGameInstance.myGameInstance_C|GetBlueWins _asmy_game_instance) 1)))
      (:then_1
        (bind _returnvalue_2 (UserInterface|CreateWidget "/Game/Sprites/p1win.p1win_C"))
        (UserInterface|Viewport|AddtoViewport _returnvalue_2 0)
        (Input|DisableInput (Game|GetPlayerController 0))
        (Input|DisableInput (Game|GetPlayerController 1)))
      (:then_2
        (Utilities|FlowControl|Delay 0.5)
        (Game|OpenLevel(byName) (Variables|Default|Getnew_level))))))

(event Custom|BulletTimer
  ;[1 1 1] Shooting
  (Utilities|FlowControl|Delay 0.2)
  (Variables|Default|SetisShooting false))

(event EventOnLanded
  (params (Hit :type Hit%20Result%20Structure%20%28by%20ref%29))
  ;[1 1 1] Changing Flipbooks/Jumping
  (Variables|Default|SetJump%20Count 0))

(event EventBeginPlay
  (Utilities|FlowControl|Sequence
    (:then_0
      ;[1 1 1] replication
      (Class|ActorComponent|SetIsReplicated (Variables|Default|GetSprite) false))
    (:then_1
      ;[1 1 1] UI
      (bind _returnvalue (UserInterface|CreateWidget "/Game/Blueprints/UI.UI_C"))
      (UserInterface|Viewport|AddtoViewport _returnvalue 0))))

(event EventTick
  (params (DeltaSeconds :type Float%20%28single-precision%29))
  (bind _output_get (Variables|Default|SetisMoving (> (Math|Vector|VectorLength (Transformation|GetVelocity)) 0.0)))
  (bind _output_get_2 (Variables|Default|SetisJumping (AI|Components|NavMovement|IsFalling (Variables|Character|GetCharacterMovement))))
  (bind _output_get_3 (Variables|Default|SetisIdle (== 0 (Math|Float|Truncate (Math|Vector|VectorLength (Transformation|GetVelocity))))))
  (CallFunction|AnimationPicker (Variables|Default|GetisShooting) _output_get_2 _output_get _output_get_3))

(event Input|ActionEvents|InputActionExitgame
  (params (Key :type Key%20Structure))
  (:Pressed
    (Game|QuitGame 0 "Quit")))

(event Input|ActionEvents|InputActionDash
  (params (Key :type Key%20Structure))
  ;[1 1 1] Testing Dashing
)

(event Input|ActionEvents|InputActionJump
  (params (Key :type Key%20Structure))
  ;[1 1 1] Changing Flipbooks/Jumping
  (:Pressed
    (if (< (Variables|Default|GetJump%20Count) 3)
      (Variables|Default|SetJump%20Count (+ (Variables|Default|GetJump%20Count) 1))
      (Character|Jump)
      (Variables|Default|SetisJumping true)))
  (:Released
    (Character|StopJumping)))

(event Input|ActionEvents|InputActionFirePlayerBullet
  (params (Key :type Key%20Structure))
  (bind _returnvalue (Transformation|GetActorLocation))
  ;[1 1 1] Shooting
  (:Pressed
    (if (Variables|Default|GetCanShoot)
      (switch int (+ (Math|Float|Truncate (Input|AxisValues|GetPointUp)) 1)
        (:0
          (Effects|SpawnEmitteratLocation "/Game/StarterContent/Particles/BulletExplosion.BulletExplosion" (Transformation|GetWorldLocation (Variables|Default|GetArrow1)) :!label _label)
          (Sprite|SetFlipbook (Variables|Default|GetSprite) "/Game/Sprites/New_Artwork_v01/Sprites/Sprites_BlueAlienShootForward/BlueAlienShootForward.BlueAlienShootForward"))
        (:1
          (goto _label))
        (:2
          (Effects|SpawnEmitteratLocation "/Game/StarterContent/Particles/BulletExplosion.BulletExplosion" (Transformation|GetWorldLocation (Variables|Default|GetArrow2)))
          (Sprite|SetFlipbook (Variables|Default|GetSprite) "/Game/Sprites/New_Artwork_v01/Sprites/Sprites_BlueAlienShootUp/BlueAlienShootUp.BlueAlienShootUp")))
      (CallFunction|FireBullet)
      (Variables|Default|SetisShooting true)
      (Variables|Default|SetbulletsLeft (- (Variables|Default|GetbulletsLeft) 1.0))
      (CallFunction|BulletTimer)
      ;[1 1 1] Reload
      (if (<= (Variables|Default|GetbulletsLeft) 0.0)
        (Utilities|FlowControl|Sequence
          (:then_0
            (Audio|PlaySoundatLocation "/Game/SoundAssets/Recharge.Recharge" _returnvalue))
          (:then_1
            (Variables|Default|SetCanShoot false)
            (bind _reload_fill (Timeline|Reload_fill PlayFromStart)
              (:Update
                (Variables|Default|SetbulletsLeft _reload_fill))
              (:Finished
                (Audio|PlaySoundatLocation "/Game/SoundAssets/guncock.guncock" _returnvalue)
                (Variables|Default|SetCanShoot true)))))))))

(event Input|AxisEvents|InputAxisMoveRight
  (params (AxisValue :type Float%20%28single-precision%29))
  ;[1 1 1] Movement
  (Pawn|Input|AddMovementInput "1.000000,0.000000,0.000000" AxisValue false)
  (Math|Float|CompareFloat AxisValue 0.0
    (:>
      (Pawn|SetControlRotation (Pawn|GetController) (Math|Rotator|MakeRotator 0.0 0.0 0.0)))
    (:<
      (Pawn|SetControlRotation (Pawn|GetController) (Math|Rotator|MakeRotator 0.0 0.0 1.8e+02)))))

(fn ConstructionScript)

(fn FireBullet
  (switch int (+ (Math|Float|Truncate (Input|AxisValues|GetPointUp)) 1)
    (:0
      (bind _returnvalue (Game|SpawnActorfromClass "/Game/Blueprints/Player1Bullets.Player1Bullets_C" (Transformation|GetWorldTransform (Variables|Default|GetArrow1)) "AlwaysSpawn" 0 0 :!label _label))
      (Audio|PlaySoundatLocation "/Game/StarterContent/Audio/Explosion02.Explosion02" (Transformation|GetActorLocation))
      (Variables|/Script/Engine.MovementComponent|SetVelocity (Variables|/Game/Blueprints/Player1Bullets.Player1Bullets_C|GetProjectileMovement _returnvalue) (Math|Vector|MakeVector (.X (Math|Vector|BreakVector (Transformation|GetComponentVelocity (Variables|/Script/Engine.MovementComponent|GetUpdatedPrimitive (Variables|/Game/Blueprints/Player1Bullets.Player1Bullets_C|GetProjectileMovement _returnvalue))))) 0.0 (.Z (Math|Vector|BreakVector (Variables|/Script/Engine.MovementComponent|GetVelocity (Variables|Character|GetCharacterMovement)))))))
    (:1
      (goto _label))
    (:2
      (bind _returnvalue_2 (Game|SpawnActorfromClass "/Game/Blueprints/Player1Bullets.Player1Bullets_C" (Transformation|GetWorldTransform (Variables|Default|GetArrow2)) "AlwaysSpawn" 0 0))
      (Audio|PlaySoundatLocation "/Game/StarterContent/Audio/Explosion02.Explosion02" (Transformation|GetActorLocation))
      (Variables|/Script/Engine.MovementComponent|SetVelocity (Variables|/Game/Blueprints/Player1Bullets.Player1Bullets_C|GetProjectileMovement _returnvalue_2) (Math|Vector|MakeVector (.X (Math|Vector|BreakVector (Variables|/Script/Engine.MovementComponent|GetVelocity (Variables|Character|GetCharacterMovement)))) 0.0 (.Z (Math|Vector|BreakVector (Transformation|GetComponentVelocity (Variables|/Script/Engine.MovementComponent|GetUpdatedPrimitive (Variables|/Game/Blueprints/Player1Bullets.Player1Bullets_C|GetProjectileMovement _returnvalue_2))))))))))

(fn AnimationPicker
  (params (shooting :type Boolean) (jumping :type Boolean) (moving :type Boolean) (idle :type Boolean))
  (bind _returnvalue (Input|AxisValues|GetPointUp))
  (bind _sprite (Variables|Default|GetSprite))
  (bind _returnvalue_2 (Math|Float|Truncate _returnvalue))
  (bind _returnvalue_3 (> _returnvalue_2 0))
  (bind _returnvalue_4 (< _returnvalue_2 0))
  (if (not shooting)
    (if jumping
      (if _returnvalue_3
        (Sprite|SetFlipbook _sprite "/Game/Sprites/New_Artwork_v01/Sprites/Sprites_BlueAlienJumpUp/BlueAlienJumpUp.BlueAlienJumpUp")
        (else
          (if _returnvalue_4
            _
            (else
              _))
          (Sprite|SetFlipbook _sprite "/Game/Sprites/New_Artwork_v01/Sprites/Sprites_BlueAlienJump/BlueAlienJump.BlueAlienJump")))
      (elif moving
        (if _returnvalue_4
          (Sprite|SetFlipbook _sprite "/Game/Sprites/New_Artwork_v01/Sprites/Sprites_BlueAlienRun/BluealienRun.BluealienRun" :!label _label)
          (elif _returnvalue_3
            (Sprite|SetFlipbook _sprite "/Game/Sprites/New_Artwork_v01/Sprites/Sprites_BlueAlienRunUp/BlueAlienRunUp.BlueAlienRunUp")
            (else
              (goto _label))))
        (elif _returnvalue_3
          (Sprite|SetFlipbook _sprite "/Game/Sprites/New_Artwork_v01/Sprites/Sprites_BlueAlienIdleUp/BlueAlienIdleUp.BlueAlienIdleUp")
          (else
            (if _returnvalue_4
              _
              (else
                _))
            (Sprite|SetFlipbook _sprite "/Game/Sprites/New_Artwork_v01/Sprites/Sprites_BlueAlienIdle/BlueAlienIdle.BlueAlienIdle")))))))

(fn CanJumpInternal
  (bind _returnvalue (|CallParentFunction))
  (return (or _returnvalue (AI|Components|NavMovement|IsFalling (Variables|Character|GetCharacterMovement)))))